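; BP_MenuController is the lobby player controller that manages menu widgets and hands game-start requests to the game mode.
; ServerInitLobby triggers client events that create the loading screen and lobby HUD, with separate events to remove them or show the lobby-to-Bloodrun screen.
; ServerUpdatePlayerList relays player-list refreshes to the HUD, and RequestServerTravel asks GM_GameLobby to travel to BloodrunDeathmatch.
; Its construction script sets game-and-UI input on non-server instances.
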(event Custom|RequestServerTravel
  (bind _returnvalue (Game|GetGameMode))
  ;[1 1 1] Server travel handling
  (if (Utilities|IsValid _returnvalue)
    (bind _asgm_game_lobby (Utilities|Casting|CastToGM_GameLobby _returnvalue))
    (Default|HandleServerTravellingtoGame _asgm_game_lobby "BloodrunDeathmatch")))

(event Custom|ServerUpdatePlayerList
  ;[1 1 1] Handle player list
  (CallFunction|ClientUpdatePlayerList))

(event Custom|ClientUpdatePlayerList
  (bind _hud (Variables|Default|GetHUD))
  ;[1 1 1] Handle player list
  (if (Utilities|IsValid _hud)
    (Default|UpdatePlayersList _hud)))

(event Custom|ClientCreateLobbyWidget
  ;[1 1 1] Lobby screen handling
  (bind _returnvalue (UserInterface|CreateWidget "/Game/Blueprints/UI/Menus/MainMenu/WBP_GameLobby.WBP_GameLobby_C" self))
  (bind _output_get (Variables|Default|SetHUD _returnvalue))
  (UserInterface|Viewport|AddtoViewport _output_get 0))

(event Custom|ClientDestroyLobbyWidget
  ;[1 1 1] Lobby screen handling
  (if (Utilities|IsValid (Variables|Default|GetHUD))
    (Widget|RemovefromParent (Variables|Default|GetHUD))
    (Variables|Default|SetHUD 0)))

(event Custom|ServerInitLobby
  ;[1 1 1] Hande HUD creation
  (CallFunction|ClientCreateLoadingWidget)
  (CallFunction|ClientCreateLobbyWidget))

(event Custom|ClientCreateLoadingWidget
  ;[1 1 1] Loading screen handling
  (bind _returnvalue (UserInterface|CreateWidget "/Game/Blueprints/UI/Transitions/WBP_LoadingScreen.WBP_LoadingScreen_C" self))
  (bind _output_get (Variables|Default|SetLoadingScreen _returnvalue))
  (UserInterface|Viewport|AddtoViewport _output_get 1))

(event Custom|ClientDestroyLoadingWidget
  ;[1 1 1] Loading screen handling
  (Widget|RemovefromParent (Variables|Default|GetLoadingScreen)))

(event Custom|ClientCreateGameLoadingWidget
  ;[1 1 1] Loading screen handling
  (bind _returnvalue (UserInterface|CreateWidget "/Game/Blueprints/UI/Transitions/WBP_LobbyToBloodrun.WBP_LobbyToBloodrun_C" self))
  (UserInterface|Viewport|AddtoViewport _returnvalue 0))

(fn ConstructionScript
  (if (not (Networking|IsServer))
    (Input|SetInputModeGameandUI self 0 "LockInFullscreen" false)))