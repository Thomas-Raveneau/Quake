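; Multiplayer player character with separate first- and third-person views, armed with rocket launchers.
; BeginPlay attaches one launcher to the arms and another to the body, splitting visibility between owner and others.
; Look-up input sends control rotation through server and multicast events to rotate the spine-aligned FPS pivot on non-local copies.
; Fire gets a transform from the first-person launcher for server rocket spawning; damage and debug health/shield keys call server functions.
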(event Custom|Server%20SyncControlRotation
  (params (Control%20Rotation :type Rotator))
  ;[1 1 1] Gun pitch replication
  (Variables|Default|SetSyncControlRotation Control%20Rotation)
  (if (not (Pawn|IsLocallyControlled))
    (Transformation|SetWorldRotation (Variables|Default|GetPivotPointFPS) (Variables|Default|GetSyncControlRotation) false false)
    (if (Ability|HasAuthority)
      (CallFunction|ServerMulticastSyncControlRotation (Variables|Default|GetSyncControlRotation)))))

(event Custom|Server%20SpawnRocketProjectile
  (params (SpawnTransform :type Transform))
  ;[1 1 1] Weapon fire
  (Game|SpawnActorfromClass "/Game/Blueprints/Weapons/RocketLauncher/BP_RocketProjectile.BP_RocketProjectile_C" SpawnTransform "Undefined" self 0))

(event Custom|Server%20Multicast%20SyncControlRotation
  (params (ControlRotation :type Rotator))
  ;[1 1 1] Gun pitch replication
  (Variables|Default|SetSyncControlRotation ControlRotation)
  (if (not (Pawn|IsLocallyControlled))
    (Transformation|SetWorldRotation (Variables|Default|GetPivotPointFPS) (Variables|Default|GetSyncControlRotation) false false)))

(event EventBeginPlay
  (Utilities|FlowControl|Sequence
    (:then_0
      ;[1 1 1] Spawn player default weapon
      (bind _returnvalue (Game|SpawnActorfromClass "/Game/Blueprints/Weapons/RocketLauncher/BP_RocketLauncher.BP_RocketLauncher_C" (Math|Transform|MakeTransform "0, 0, 0" "0, 0, 0" "1,1,1") "Undefined" self 0))
      (Variables|Default|SetWeaponFP _returnvalue)
      (bind _returnvalue_2 (Game|SpawnActorfromClass "/Game/Blueprints/Weapons/RocketLauncher/BP_RocketLauncher.BP_RocketLauncher_C" (Math|Transform|MakeTransform "0, 0, 0" "0, 0, 0" "1,1,1") "Undefined" self 0))
      (Variables|Default|SetWeaponTP _returnvalue_2))
    (:then_1
      ;[1 1 1] Attach weapons to arms and body
      (Transformation|AttachComponentToComponent (Variables|Default|GetWeaponFP) (Variables|Default|GetArmsFPS) "GripPointFPS" "SnapToTarget" "SnapToTarget" "SnapToTarget" true)
      (Transformation|AttachComponentToComponent (Variables|Default|GetWeaponTP) (Variables|Default|GetBody) "GripPoint" "KeepRelative" "KeepRelative" "KeepRelative" true))
    (:then_2
      ;[1 1 1] Define first person visibility
      (Rendering|SetOnlyOwnerSee (Variables|/Game/Blueprints/Weapons/RocketLauncher/BP_RocketLauncher.BP_RocketLauncher_C|GetSK_RocketLauncher (.AsBP%20Rocket%20Launcher (Utilities|Casting|CastToBP_RocketLauncher (Variables|Default|GetWeaponFP)))) true :!class /Script/Engine.PrimitiveComponent)
      (Rendering|SetOnlyOwnerSee (Variables|Default|GetArmsFPS) true :!class /Script/Engine.PrimitiveComponent)
      ;[1 1 1] Set third person visibility
      (Class|PrimitiveComponent|SetOwnerNoSee (Variables|/Game/Blueprints/Weapons/RocketLauncher/BP_RocketLauncher.BP_RocketLauncher_C|GetSK_RocketLauncher (.AsBP%20Rocket%20Launcher (Utilities|Casting|CastToBP_RocketLauncher (Variables|Default|GetWeaponTP)))) true)
      (Class|PrimitiveComponent|SetOwnerNoSee (Variables|Default|GetBody) true))))

(event Game|Damage|EventRadialDamage
  (params (DamageReceived :type Float%20%28single-precision%29) (DamageType :type Damage%20Type%20Object%20Reference) (Origin :type Vector :default "0, 0, 0") (HitInfo :type Hit%20Result%20Structure%20%28by%20ref%29) (InstigatedBy :type Controller%20Object%20Reference) (DamageCauser :type Actor%20Object%20Reference))
  ;[1 1 1] Handle recevied damages
  ;;[1 1 1] Handle explosion damages
  (Class|QuakePlayer|ServerTakeDamage (Math|Float|Truncate DamageReceived) InstigatedBy DamageCauser))

(event Game|Damage|EventPointDamage
  (params (Damage :type Float%20%28single-precision%29) (DamageType :type Damage%20Type%20Object%20Reference) (HitLocation :type Vector :default "0, 0, 0") (HitNormal :type Vector :default "0, 0, 0") (HitComponent :type Primitive%20Component%20Object%20Reference) (BoneName :type Name :default "None") (ShotFromDirection :type Vector :default "0, 0, 0") (InstigatedBy :type Controller%20Object%20Reference) (DamageCauser :type Actor%20Object%20Reference) (HitInfo :type Hit%20Result%20Structure%20%28by%20ref%29))
  ;[1 1 1] Handle recevied damages
  ;;[1 1 1] Handle classic damage
  (Class|QuakePlayer|ServerTakeDamage (Math|Float|Truncate Damage) InstigatedBy DamageCauser))

(event Input|ActionEvents|InputActionFire
  (params (Key :type Key%20Structure :default "None"))
  (bind _camerafps (Variables|Camera|GetCameraFPS))
  ;[1 1 1] Weapon fire
  (:Pressed
    (bind _returnvalue (Class|Weapon|Shoot (Variables|Default|GetWeaponFP) (Math|Vector|GetForwardVector _camerafps) (Transformation|GetWorldRotation _camerafps)))
    (CallFunction|ServerSpawnRocketProjectile _returnvalue)))

(event Input|AxisEvents|InputAxisLookUp
  (params (AxisValue :type Float%20%28single-precision%29))
  ;[1 1 1] Look up event
  (Pawn|Input|AddControllerPitchInput AxisValue)
  (if (Pawn|IsLocallyControlled)
    (CallFunction|ServerSyncControlRotation (Pawn|GetControlRotation :!class /Script/Engine.Pawn))))

(event Input|KeyboardEvents|Down
  (params (Key :type Key%20Structure :default "None"))
  ;[1 0.04076 0.08056] Debug Health and Shield stats
  (:Pressed
    (Class|QuakePlayer|ServerSubstractHealth 50)))

(event Input|KeyboardEvents|Up
  (params (Key :type Key%20Structure :default "None"))
  ;[1 0.04076 0.08056] Debug Health and Shield stats
  (:Pressed
    (Class|QuakePlayer|ServerAddHealth 50)))

(event Input|KeyboardEvents|Right
  (params (Key :type Key%20Structure :default "None"))
  ;[1 0.04076 0.08056] Debug Health and Shield stats
  (:Pressed
    (Class|QuakePlayer|ServerAddShield 50)))

(event Input|KeyboardEvents|Left
  (params (Key :type Key%20Structure :default "None"))
  ;[1 0.04076 0.08056] Debug Health and Shield stats
  (:Pressed
    (Class|QuakePlayer|ServerSubstractShield 50)))

(fn ConstructionScript
  (Utilities|FlowControl|Sequence
    (:then_0
      ;[1 1 1] Set FPSPivotPoint location to spine_01 location
      (Transformation|SetWorldLocation (Variables|Default|GetPivotPointFPS) (Transformation|GetSocketLocation (Variables|Default|GetBody) "spine_01") false false))))