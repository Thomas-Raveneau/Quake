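; Rocket launcher projectile that explodes once on its first hit, or on overlap with an actor other than its owner.
; MulticastExplode hides the mesh, plays sound and particles, fires a RadialForce impulse, and applies radial damage credited to the owning BP_Player's controller.
; ExplosionRadius drives both force and damage radii, and ServerDestroyRocket destroys the actor when the particles finish.
; A separate Explode function with hardcoded damage values is not called here.
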(event OnComponentHit(SM_Rocket)
  (params (HitComponent :type Primitive%20Component%20Object%20Reference) (OtherActor :type Actor%20Object%20Reference) (OtherComp :type Primitive%20Component%20Object%20Reference) (NormalImpulse :type Vector :default "0, 0, 0") (Hit :type Hit%20Result%20Structure%20%28by%20ref%29))
  ;[1 1 1] Rocket collision detection
  (if (not (Variables|Default|GetCollided))
    (Variables|Default|SetCollided true)
    (CallFunction|MulticastExplode)))

(event OnComponentBeginOverlap(SM_Rocket)
  (params (OverlappedComponent :type Primitive%20Component%20Object%20Reference) (OtherActor :type Actor%20Object%20Reference) (OtherComp :type Primitive%20Component%20Object%20Reference) (OtherBodyIndex :type Integer) (bFromSweep :type Boolean) (SweepResult :type Hit%20Result%20Structure%20%28by%20ref%29))
  ;[1 1 1] Rocket collision detection
  (if (and (!= OtherActor (Components|GetOwner)) (not (Variables|Default|GetCollided)))
    (Variables|Default|SetCollided true)
    (CallFunction|MulticastExplode)))

(event Custom|Multicast%20Explode
  (bind _returnvalue (Transformation|GetActorTransform))
  (bind _radialforce (Variables|Default|GetRadialForce))
  ;[1 1 1] Explosion handling
  (Variables|/Script/Engine.ProjectileMovementComponent|SetMaxSpeed (Variables|Default|GetProjectileMovement) 0.0)
  (Audio|PlaySoundatLocation "/Game/Assets/Sounds/Effects/Rocket/Explosion_Cue.Explosion_Cue" (Transformation|GetActorLocation) "0, 0, 0" 0.3 1.0 0.0 0 0 self)
  (bind _returnvalue_2 (Effects|SpawnEmitteratLocation "/Game/Assets/Effects/P_Explosion.P_Explosion" (.location _returnvalue) (.rotation _returnvalue) "1.000000,1.000000,1.000000" false "ManualRelease"))
  (Development|SetHiddeninGame (Variables|Default|GetSM_Rocket) true true)
  (if (Utilities|IsValid _returnvalue_2)
    (EventDispatchers|AssignOnSystemFinished _returnvalue_2 (delegate Custom|OnExplosionFinished)))
  (Utilities|FlowControl|Sequence
    (:then_0
      (Utilities|IsValid _radialforce
        (:Is%20Valid
          (Class|RadialForceComponent|FireImpulse _radialforce))))
    (:then_1
      (bind _asbp_player (Utilities|Casting|CastToBP_Player (Components|GetOwner))
        (:then
          (if (Utilities|IsValid _asbp_player)
            (Game|Damage|ApplyRadialDamage (Math|Conversions|ToFloat(Integer) (Variables|Default|GetRocketDamage)) (Transformation|GetActorLocation) (Variables|Default|GetExplosionRadius) 0 0 self (Pawn|GetController _asbp_player) false "ECC_Visibility")))
        (:CastFailed
          (Development|PrintString "Cast failed"))))))

(event Custom|OnExplosionFinished
  (params (PSystem :type Particle%20System%20Component%20Object%20Reference))
  ;[1 1 1] Explosion handling
  (CallFunction|ServerDestroyRocket))

(event Custom|Server%20DestroyRocket
  ;[1 1 1] Destroying rocket when explosion particle ended
  (Actor|DestroyActor))

(fn ConstructionScript
  (Variables|/Script/Engine.RadialForceComponent|SetRadius (Variables|Default|GetRadialForce) (Variables|Default|GetExplosionRadius)))

(fn Explode
  (bind _returnvalue (Transformation|GetActorTransform))
  (bind _radialforce (Variables|Default|GetRadialForce))
  (Audio|PlaySoundatLocation "/Game/Assets/Sounds/Effects/Rocket/Explosion_Cue.Explosion_Cue" (Transformation|GetActorLocation) "0, 0, 0" 0.3 1.0 0.0 0 0 self)
  (Effects|SpawnEmitteratLocation "/Game/Assets/Effects/P_Explosion.P_Explosion" (.location _returnvalue) (.rotation _returnvalue))
  (Utilities|FlowControl|Sequence
    (:then_0
      (Utilities|IsValid _radialforce
        (:Is%20Valid
          (Class|RadialForceComponent|FireImpulse _radialforce))))
    (:then_1
      (Game|Damage|ApplyRadialDamage 1e+02 (Transformation|GetActorLocation) 225.0 0 0 self 0 false "ECC_Visibility"))))