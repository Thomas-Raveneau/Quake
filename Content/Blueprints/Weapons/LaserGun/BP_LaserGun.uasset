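; BP_LaserGun is the player's laser weapon, flagged on BeginPlay as an instant-shoot weapon through a server call.
; Tick polls the owning BP_Player's IsShootingLaser to start or stop the looping fire sound, which also stops on EndPlay.
; Events play swap and fire cues, with CanShoot set true when the swap audio finishes.
; It also sets first- or third-person mesh visibility and returns the muzzle socket location.
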(event OnAudioFinished(Swap_Cue)
  (Variables|Default|SetCanShoot true))

(event Custom|StopFireLoopSound
  (Audio|Components|Audio|Stop (Variables|Default|GetFireLoop_Cue)))

(event EventSetWeaponVisibility
  (params (FPSView :type Boolean))
  ;[1 1 1] Handle weapon visibility
  (if FPSView
    (Rendering|SetOnlyOwnerSee (Variables|Default|GetSK_LaserGun) true :!class /Script/Engine.PrimitiveComponent)
    (else
      (Class|PrimitiveComponent|SetOwnerNoSee (Variables|Default|GetSK_LaserGun) true))))

(event EventPlayFireSound
  (Audio|Components|Audio|Play (Variables|Default|GetFire_Cue) 0.0))

(event EventPlayWeaponSwapSound
  (Audio|Components|Audio|Play (Variables|Default|GetSwap_Cue) 0.0))

(event EventEndPlay
  (params (EndPlayReason :type EEndPlayReason%20Enum :default "Destroyed"))
  (CallFunction|StopFireLoopSound))

(event EventBeginPlay
  ;[1 1 1] Handle construction
  (Class|Weapon|ServerSetInstantShootWeapon true)
  (bind _asbp_player (Utilities|Casting|CastToBP_Player (Components|GetOwner)))
  (Variables|Default|SetPlayerOwner _asbp_player))

(event EventTick
  (params (DeltaSeconds :type Float%20%28single-precision%29))
  ;[1 1 1] Handle fire loop sound if owner is shooting laser
  (Utilities|FlowControl|Sequence
    (:then_0
      (if (and (Variables|/Script/Quake.QuakePlayer|GetIsShootingLaser (Variables|Default|GetPlayerOwner)) (not (Audio|Components|Audio|IsPlaying (Variables|Default|GetFireLoop_Cue))))
        (Audio|Components|Audio|Play (Variables|Default|GetFireLoop_Cue) 0.0)))
    (:then_1
      (if (and (not (Variables|/Script/Quake.QuakePlayer|GetIsShootingLaser (Variables|Default|GetPlayerOwner))) (Audio|Components|Audio|IsPlaying (Variables|Default|GetFireLoop_Cue)))
        (CallFunction|StopFireLoopSound)))))

(fn ConstructionScript)

(fn GetMuzzleLocation
  (return (Transformation|GetSocketLocation (Variables|Default|GetSK_LaserGun) "Muzzle_Bone")))