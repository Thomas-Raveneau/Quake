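; Laser beam actor for a weapon, owned by BP_Player, that deals continuous point damage along its forward line.
; Each tick a Camera-channel line trace sets the Niagara beam's end point, shows the impact effect on blocking hits, and damages the hit actor.
; Impact placement and damage require the BP_Player owner cast to succeed.
; StopLaser runs once, deactivating both effects and playing a timeline on beam scale before destroying the actor.
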(event Custom|StopLaser
  (Utilities|FlowControl|DoOnce false
    (:Completed
      (Components|Activation|Deactivate (Variables|Default|GetNiagaraLaser))
      (Components|Activation|Deactivate (Variables|Default|GetNiagaraLaserImpact))
      (bind _scale (Timeline|StopLaserEffect PlayFromStart)
        (:Update
          (Effects|Components|ParticleSystem|SetFloatParameter (Variables|Default|GetNiagaraLaser) "Scale" _scale))
        (:Finished
          (Actor|DestroyActor))))))

(event EventBeginPlay
  (Effects|Components|ParticleSystem|SetColorParameter (Variables|Default|GetNiagaraLaser) "Color" "(R=0.000000,G=0.616949,B=0.979167,A=1.000000)")
  (Effects|Components|ParticleSystem|SetColorParameter (Variables|Default|GetNiagaraLaserImpact) "Color" "(R=0.251593,G=0.565973,B=1.000000,A=1.000000)"))

(event Collision|EventActorBeginOverlap
  (params (OtherActor :type Actor%20Object%20Reference)))

(event EventTick
  (params (DeltaSeconds :type Float%20%28single-precision%29))
  (bind _returnvalue (Transformation|GetActorLocation))
  (bind _returnvalue_2 (Transformation|GetActorForwardVector))
  (bind _distance (Variables|Default|GetDistance))
  (bind _returnvalue_3 (* _returnvalue_2 _distance))
  (bind _returnvalue_4 (+ _returnvalue _returnvalue_3))
  (Variables|Default|SetTraceEnd _returnvalue_4)
  (bind _outhit (Collision|LineTraceByChannel _returnvalue _returnvalue_4 "TraceTypeQuery2" false 0 "ForOneFrame"))
  (Variables|Default|SetOut%20Hit _outhit)
  (Variables|Default|SetBlocking%20Hit (.bBlockingHit (Collision|BreakHitResult _outhit)))
  (Variables|Default|SetHit%20Actor (.HitActor (Collision|BreakHitResult _outhit)))
  (Variables|Default|SetLocation (.Location (Collision|BreakHitResult _outhit)))
  (Effects|Components|ParticleSystem|SetVectorParameter (Variables|Default|GetNiagaraLaser) "LaserEnd" (select (Variables|Default|GetBlocking%20Hit) (Variables|Default|GetLocation) (Variables|Default|GetTraceEnd)))
  (Rendering|SetVisibility (Variables|Default|GetNiagaraLaserImpact) (Variables|Default|GetBlocking%20Hit) false)
  (bind _asbp_player (Utilities|Casting|CastToBP_Player (Components|GetOwner))
    (:then
      (Transformation|SetWorldLocation (Variables|Default|GetNiagaraLaserImpact) (Variables|Default|GetLocation) false false)
      (Game|Damage|ApplyPointDamage (Variables|Default|GetHit%20Actor) (Math|Conversions|ToFloat(Integer) (Variables|Default|GetLaserDamage)) (Variables|Default|GetLocation) (Variables|Default|GetOut%20Hit) (Pawn|GetController _asbp_player) self))
    (:CastFailed
      (Development|PrintString "Laser Fail to cast to Player"))))

(fn ConstructionScript)