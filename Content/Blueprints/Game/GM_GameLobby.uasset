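; GM_GameLobby is the lobby game mode that tracks connected players and handles travel from the lobby to a map.
; Login adds each BP_MenuController to PlayersInLobby and calls its ServerInitLobby, while logout removes it.
; UpdatePlayersList calls ServerUpdatePlayerList on every tracked controller, running before the add on login and after the removal on logout.
; TravelTo runs a servertravel console command with the given map name appended.
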(event Custom|TravelTo
  (params (MapName :type String))
  ;[1 1 1] Lobby server travel handling
  (Development|ExecuteConsoleCommand (Utilities|String|Append "servertravel " MapName) 0))

(event Custom|UpdatePlayersList
  ;[1 1 1] Update player list widgets
  (for _array_element (Variables|Default|GetPlayersInLobby)
    (Default|ServerUpdatePlayerList _array_element)))

(event EventPostLogin
  (params (NewPlayer :type Player%20Controller%20Object%20Reference))
  ;[1 1 1] Login handling
  (CallFunction|UpdatePlayersList)
  (bind _asbp_menu_controller (Utilities|Casting|CastToBP_MenuController NewPlayer))
  (Utilities|Array|AddUnique (Variables|Default|GetPlayersInLobby) _asbp_menu_controller)
  (Default|ServerInitLobby _asbp_menu_controller))

(event EventOnLogout
  (params (ExitingController :type Controller%20Object%20Reference))
  ;[1 1 1] Logout handling
  (bind _asbp_menu_controller (Utilities|Casting|CastToBP_MenuController ExitingController))
  (Utilities|Array|RemoveItem (Variables|Default|GetPlayersInLobby) _asbp_menu_controller)
  (CallFunction|UpdatePlayersList))

(fn ConstructionScript)